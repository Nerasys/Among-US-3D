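; Electrical panel actor for an Among Us-style game that handles the lights sabotage and its repair.
; On shutdown it switches its monitors and turns off every BP_Light, giving crewmates a flashlight, while impostors get a separate light mode.
; During an outage, a trigger lets the local player press use, through a bound event and gate, to start repairing.
; LightsRepair restores monitors and lights and removes the flashlight.
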(event `self.Trigger_LightsEnable.OnComponentBeginOverlap`
  (params (OverlappedComponent :type "PrimitiveComponent Object Reference") (OtherActor :type "Actor Object Reference") (OtherComp :type "PrimitiveComponent Object Reference") (OtherBodyIndex :type Integer) (bFromSweep :type Boolean) (SweepResult :type "HitResult Structure (by ref)"))
  ;[1 1 1] Input
  (if (`self.ElectricityShutdown`)
    (if (== OtherActor (`GameplayStatics.GetPlayerPawn` 0))
      (bind _asbp_first_person_character (cast `/Game/FirstPerson/Blueprints/BP_FirstPersonCharacter` (`GameplayStatics.GetPlayerPawn` 0)))
      (set `/Game/FirstPerson/Blueprints/BP_FirstPersonCharacter.CanRepairLights` true _asbp_first_person_character)
      (add `/Game/FirstPerson/Blueprints/BP_FirstPersonCharacter.InputUse` _asbp_first_person_character (delegate `InputUse`))
      (goto _label :!via `Open`))))

(event `InputUse`
  ;[1 1 1] Input
  (`/Engine/EditorBlueprintResources/StandardMacros.Gate` true :!label _label
    (:`Exit`
      (if (`self.ElectricityShutdown`)
        (bind _asbp_first_person_character (cast `/Game/FirstPerson/Blueprints/BP_FirstPersonCharacter` (`GameplayStatics.GetPlayerPawn` 0)))
        (`/Game/FirstPerson/Blueprints/BP_FirstPersonCharacter.RepairLightsPlayer` _asbp_first_person_character)))))

(event `self.Trigger_LightsEnable.OnComponentEndOverlap`
  (params (OverlappedComponent :type "PrimitiveComponent Object Reference") (OtherActor :type "Actor Object Reference") (OtherComp :type "PrimitiveComponent Object Reference") (OtherBodyIndex :type Integer))
  ;[1 1 1] Input
  (if (`self.ElectricityShutdown`)
    (if (== OtherActor (`GameplayStatics.GetPlayerPawn` 0))
      (bind _asbp_first_person_character (cast `/Game/FirstPerson/Blueprints/BP_FirstPersonCharacter` (`GameplayStatics.GetPlayerPawn` 0)))
      (set `/Game/FirstPerson/Blueprints/BP_FirstPersonCharacter.CanRepairLights` false _asbp_first_person_character)
      (goto _label :!via `Close`))))

(event `LightsShutdown`
  ;[1 1 1] Lights Shutdown
  (set `self.ElectricityShutdown` true)
  (`PrimitiveComponent.SetMaterial` (`self.Screen1`) 0 "/Game/Amogus/Materials/MT_Monitor_ON.MT_Monitor_ON")
  (`PrimitiveComponent.SetMaterial` (`self.Screen`) 0 "/Game/Amogus/Materials/MT_Monitor_ON.MT_Monitor_ON")
  (bind _asbp_first_person_character (cast `/Game/FirstPerson/Blueprints/BP_FirstPersonCharacter` (`GameplayStatics.GetPlayerCharacter` 0)))
  (if (`/Game/FirstPerson/Blueprints/BP_FirstPersonCharacter.IsImpostor` _asbp_first_person_character)
    (bind _outactors (`GameplayStatics.GetAllActorsOfClass` "/Game/Amogus/Blueprints/BP_Light.BP_Light_C"))
    (for _array_element _outactors
      (`/Game/Amogus/Blueprints/BP_Light.LightsImpostor` _array_element))
    (else
      (bind _outactors_2 (`GameplayStatics.GetAllActorsOfClass` "/Game/Amogus/Blueprints/BP_Light.BP_Light_C"))
      (for _array_element_2 _outactors_2
        (`/Game/Amogus/Blueprints/BP_Light.LightOff` _array_element_2))
      (`/Game/FirstPerson/Blueprints/BP_FirstPersonCharacter.ActivateLampeDePoche` _asbp_first_person_character))))

(event `LightsRepair`
  ;[1 1 1] Lights repair
  (set `self.ElectricityShutdown` false)
  (`PrimitiveComponent.SetMaterial` (`self.Screen1`) 0 "/Game/Amogus/Materials/MT_Monitor_GREEN.MT_Monitor_GREEN")
  (`PrimitiveComponent.SetMaterial` (`self.Screen`) 0 "/Game/Amogus/Materials/MT_Monitor_GREEN.MT_Monitor_GREEN")
  (bind _outactors (`GameplayStatics.GetAllActorsOfClass` "/Game/Amogus/Blueprints/BP_Light.BP_Light_C"))
  (for _array_element _outactors
    (`/Game/Amogus/Blueprints/BP_Light.LightOn` _array_element))
  (bind _asbp_first_person_character (cast `/Game/FirstPerson/Blueprints/BP_FirstPersonCharacter` (`GameplayStatics.GetPlayerCharacter` 0)))
  (`/Game/FirstPerson/Blueprints/BP_FirstPersonCharacter.DesactivateLampeDePoche` _asbp_first_person_character))

(fn `UserConstructionScript`)