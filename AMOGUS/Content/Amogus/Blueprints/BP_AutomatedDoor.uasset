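; BP_AutomatedDoor is a door that opens automatically when actors overlap it and closes once all have left.
; An overlap counter tracks occupants, and an IsOpen flag blocks repeat openings while MoveComponentTo slides the Door component up.
; After a hold delay it polls the counter until empty, lowers the door, and reopens if someone entered during closing.
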(event `self.ReceiveActorBeginOverlap`
  (params (OtherActor :type "Actor Object Reference"))
  (bind _door (`self.Door`))
  (bind _door_2 (`self.Door`))
  (`/Engine/EditorBlueprintResources/StandardMacros.IncrementInt` (`self.NbOfActors`)
    (:`  `
      (if (not (`self.IsOpen`)) :!label _label
        (set `self.IsOpen` true)
        (`KismetSystemLibrary.MoveComponentTo` _door (+ (`SceneComponent.RelativeLocation` _door) (0.0 0.0 350.0)) (struct) false false 0.6)
        (`KismetSystemLibrary.Delay` 2.0)
        (if (== (`self.NbOfActors`) 0) :!label _label_2
          (`KismetSystemLibrary.MoveComponentTo` _door_2 (+ (`SceneComponent.RelativeLocation` _door_2) (0.0 0.0 -350.0)) (struct) false false 0.6)
          (`KismetSystemLibrary.Delay` 0.4)
          (set `self.IsOpen` false)
          (if (not (== (`self.NbOfActors`) 0))
            (goto _label))
          (else
            (`KismetSystemLibrary.Delay` 0.5)
            (goto _label_2)))))))

(event `self.ReceiveActorEndOverlap`
  (params (OtherActor :type "Actor Object Reference"))
  (`/Engine/EditorBlueprintResources/StandardMacros.DecrementInt` (`self.NbOfActors`)))

(fn `UserConstructionScript`)