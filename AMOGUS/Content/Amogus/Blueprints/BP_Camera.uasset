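; BP_Camera is a security camera actor that shows whether it is being monitored.
; Every Tick it reads the IsMonitored flag, then sets the Monitor's material to its on or off version and the TEXT component to "CAM ON" or "CAM OFF".
; The file only reads IsMonitored and never sets it, and the display is reapplied each frame rather than on change.
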(event `self.ReceiveTick`
  (params (DeltaSeconds :type "Float (single-precision)"))
  (bind _text (`self.TEXT`))
  (if (`self.IsMonitored`)
    (`PrimitiveComponent.SetMaterial` (`self.Monitor`) 0 "/Game/Amogus/Materials/MT_Monitor_ON.MT_Monitor_ON")
    (`TextRenderComponent.K2_SetText` _text "CAM \nON")
    (else
      (`PrimitiveComponent.SetMaterial` (`self.Monitor`) 0 "/Game/Amogus/Materials/MT_Monitor_OFF.MT_Monitor_OFF")
      (`TextRenderComponent.K2_SetText` _text "CAM \nOFF"))))

(fn `UserConstructionScript`)