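; Dead body actor for an Among Us-style game that the player can report while standing near it.
; Its box trigger sets CanReport on the first-person character as player pawn 0 enters or leaves, and binds to the character's use input on entry.
; A Gate opened and closed by the overlaps filters that input, so reporting only works inside the box and currently just prints "REPORT".
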(event `self.BoxTrigger.OnComponentBeginOverlap`
  (params (OverlappedComponent :type "PrimitiveComponent Object Reference") (OtherActor :type "Actor Object Reference") (OtherComp :type "PrimitiveComponent Object Reference") (OtherBodyIndex :type Integer) (bFromSweep :type Boolean) (SweepResult :type "HitResult Structure (by ref)"))
  (if (== OtherActor (`GameplayStatics.GetPlayerPawn` 0))
    (bind _asbp_first_person_character (cast `/Game/FirstPerson/Blueprints/BP_FirstPersonCharacter` (`GameplayStatics.GetPlayerPawn` 0)))
    (set `/Game/FirstPerson/Blueprints/BP_FirstPersonCharacter.CanReport` true _asbp_first_person_character)
    (add `/Game/FirstPerson/Blueprints/BP_FirstPersonCharacter.InputUse` _asbp_first_person_character (delegate `InputUse`))
    (goto _label :!via `Open`)))

(event `InputUse`
  (`/Engine/EditorBlueprintResources/StandardMacros.Gate` true :!label _label
    (:`Exit`
      (`KismetSystemLibrary.PrintString` "REPORT"))))

(event `self.BoxTrigger.OnComponentEndOverlap`
  (params (OverlappedComponent :type "PrimitiveComponent Object Reference") (OtherActor :type "Actor Object Reference") (OtherComp :type "PrimitiveComponent Object Reference") (OtherBodyIndex :type Integer))
  (if (== OtherActor (`GameplayStatics.GetPlayerPawn` 0))
    (bind _asbp_first_person_character (cast `/Game/FirstPerson/Blueprints/BP_FirstPersonCharacter` (`GameplayStatics.GetPlayerPawn` 0)))
    (set `/Game/FirstPerson/Blueprints/BP_FirstPersonCharacter.CanReport` false _asbp_first_person_character)
    (goto _label :!via `Close`)))

(fn `UserConstructionScript`)