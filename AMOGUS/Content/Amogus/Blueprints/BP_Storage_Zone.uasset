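; BP_Storage_Zone is a delivery zone actor that collects storage boxes for a task.
; When an actor tagged "storagebox" begins overlapping its StorageCollisionBox, the zone destroys it and increments TotalBoxesStored.
; Once the count reaches TargetBoxes, it sets TaskCompleted, after which further overlaps are ignored.
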(event `self.StorageCollisionBox.OnComponentBeginOverlap`
  (params (OverlappedComponent :type "PrimitiveComponent Object Reference") (OtherActor :type "Actor Object Reference") (OtherComp :type "PrimitiveComponent Object Reference") (OtherBodyIndex :type Integer) (bFromSweep :type Boolean) (SweepResult :type "HitResult Structure (by ref)"))
  ;[1 1 1] Storage boxes destruction
  (if (`self.TaskCompleted`)
    _
    (elif (`self.ActorHasTag` OtherActor "storagebox")
      (`self.K2_DestroyActor` OtherActor)
      (bind _result (`/Engine/EditorBlueprintResources/StandardMacros.IncrementInt` (`self.TotalBoxesStored`))
        (:`  `
          (if (== _result (`self.TargetBoxes`))
            (set `self.TaskCompleted` true)))))))

(fn `UserConstructionScript`)