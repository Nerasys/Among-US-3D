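; BP_Light is a light fixture actor with inner and outer light components, LightIn and LightOut, that other logic switches between states.
; LightOn shows both lights in warm white, and LightOff hides them.
; LightsImpostor tints both lights dark red without changing their visibility, apparently as an impostor signal.
; The Blueprint runs no logic of its own beyond these three custom events.
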(event `LightsImpostor`
  (`LightComponent.SetLightColor` (`self.LightIn`) (struct :`R` 0.617207 :`A` 1.0) true)
  (`LightComponent.SetLightColor` (`self.LightOut`) (struct :`R` 0.617207 :`A` 1.0) true))

(event `LightOff`
  (`SceneComponent.SetVisibility` (`self.LightIn`) false false)
  (`SceneComponent.SetVisibility` (`self.LightOut`) false false))

(event `LightOn`
  (bind _lightout (`self.LightOut`))
  (bind _lightin (`self.LightIn`))
  (`SceneComponent.SetVisibility` _lightin true false)
  (`SceneComponent.SetVisibility` _lightout true false)
  (`LightComponent.SetLightColor` _lightin (struct :`R` 1.0 :`G` 0.964706 :`B` 0.831373 :`A` 1.0) true)
  (`LightComponent.SetLightColor` _lightout (struct :`R` 1.0 :`G` 0.964706 :`B` 0.831373 :`A` 1.0) true))

(fn `UserConstructionScript`)