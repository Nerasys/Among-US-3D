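; BP_Vent is a two-way vent that lets impostor players teleport between an interior and an exterior point.
; Overlapping Trigger_Interior or Trigger_Exterior casts the actor to BP_FirstPersonCharacter and checks IsImpostor.
; Impostors teleport to the matching TPInterior or TPExterior location with rotation unchanged, while other characters only get a printed refusal message.
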(event `self.Trigger_Interior.OnComponentBeginOverlap`
  (params (OverlappedComponent :type "PrimitiveComponent Object Reference") (OtherActor :type "Actor Object Reference") (OtherComp :type "PrimitiveComponent Object Reference") (OtherBodyIndex :type Integer) (bFromSweep :type Boolean) (SweepResult :type "HitResult Structure (by ref)"))
  (bind _asbp_first_person_character (cast `/Game/FirstPerson/Blueprints/BP_FirstPersonCharacter` OtherActor))
  (if (`/Game/FirstPerson/Blueprints/BP_FirstPersonCharacter.IsImpostor` _asbp_first_person_character)
    (`self.K2_TeleportTo` OtherActor (`SceneComponent.K2_GetComponentLocation` (`self.TP_Interior`)) (`self.K2_GetActorRotation` OtherActor))
    (else
      (`KismetSystemLibrary.PrintString` "Only sus people can use vents" true true (struct :`R` 0.635417 :`B` 0.01941 :`A` 1.0)))))

(event `self.Trigger_Exterior.OnComponentBeginOverlap`
  (params (OverlappedComponent :type "PrimitiveComponent Object Reference") (OtherActor :type "Actor Object Reference") (OtherComp :type "PrimitiveComponent Object Reference") (OtherBodyIndex :type Integer) (bFromSweep :type Boolean) (SweepResult :type "HitResult Structure (by ref)"))
  (bind _asbp_first_person_character (cast `/Game/FirstPerson/Blueprints/BP_FirstPersonCharacter` OtherActor))
  (if (`/Game/FirstPerson/Blueprints/BP_FirstPersonCharacter.IsImpostor` _asbp_first_person_character)
    (`self.K2_TeleportTo` OtherActor (`SceneComponent.K2_GetComponentLocation` (`self.TP_Exterior`)) (`self.K2_GetActorRotation` OtherActor))
    (else
      (`KismetSystemLibrary.PrintString` "Only sus people can use vents" true true (struct :`R` 0.635417 :`B` 0.01941 :`A` 1.0)))))

(fn `UserConstructionScript`)